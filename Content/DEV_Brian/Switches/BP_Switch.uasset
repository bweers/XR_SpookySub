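; BP_Switch is a toggle switch that flips when a component attached to a motion controller overlaps its Box.
; A DoOnce that resets after a short delay debounces the overlap.
; SetState stores SwitchState and tilts the Cylinder to match.
; BeginPlay starts it off and gives the Sphere a dynamic material, whose LightColor Tick sets every frame to OnColor or near-black according to state.
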(event `self.ReceiveBeginPlay`
  (`self.SetState` false)
  (bind _returnvalue (`PrimitiveComponent.CreateDynamicMaterialInstance` (`self.Sphere`) 0 "/Game/DEV_Brian/Switches/MAT_SwitchLight_Inst.MAT_SwitchLight_Inst" "None"))
  (bind _output_get (set `self.DynamicMaterialRef` _returnvalue))
  (`KismetSystemLibrary.PrintString` (`KismetSystemLibrary.GetDisplayName` _output_get)))

(event `self.Box.OnComponentBeginOverlap`
  (params (OverlappedComponent :type "PrimitiveComponent Object Reference") (OtherActor :type "Actor Object Reference") (OtherComp :type "PrimitiveComponent Object Reference") (OtherBodyIndex :type Integer) (bFromSweep :type Boolean) (SweepResult :type "HitResult Structure (by ref)"))
  (`|ExecutionSequence`
    (:`then_0`
      (`/Engine/EditorBlueprintResources/StandardMacros.DoOnce` false :!label _label
        (:`Completed`
          (cast `MotionControllerComponent` (`SceneComponent.GetAttachParent` OtherComp)
            (:`then`
              (if (`self.SwitchState`)
                (`self.SetState` false)
                (else
                  (`self.SetState` true))))
            (:`CastFailed`
              (`KismetSystemLibrary.PrintString` "CAST FAILED" true true (struct :`R` 1.0 :`B` 0.038757 :`A` 1.0)))))))
    (:`then_1`
      (`KismetSystemLibrary.Delay` 0.25)
      (goto _label :!via `Reset`))))

(event `self.ReceiveTick`
  (params (DeltaSeconds :type "Float (single-precision)"))
  (if (`self.SwitchState`)
    (`MaterialInstanceDynamic.SetVectorParameterValue` (`self.DynamicMaterialRef`) "LightColor" (`self.OnColor`))
    (else
      (`MaterialInstanceDynamic.SetVectorParameterValue` (`self.DynamicMaterialRef`) "LightColor" (struct :`R` 0.005208 :`G` 0.005208 :`B` 0.005208 :`A` 1.0)))))

(fn `SetState`
  (params (`New State` :type Boolean))
  (bind _output_get (set `self.SwitchState` `New State`))
  (if _output_get
    (`SceneComponent.K2_SetRelativeRotation` (`self.Cylinder`) (struct :`Pitch` 20.0) false false)
    (else
      (`SceneComponent.K2_SetRelativeRotation` (`self.Cylinder`) (struct :`Pitch` -20.0) false false))))

(fn `UserConstructionScript`)