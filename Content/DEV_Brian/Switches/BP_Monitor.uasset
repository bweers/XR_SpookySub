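; BP_Monitor is a screen prop that can switch a fish scene video on and off.
; On BeginPlay it creates a dynamic material on the mesh's second slot and opens the fish scene video source.
; Events toggle the FishSceneActive material parameter, and activating the scene also plays a fish alarm sound at the monitor's location.
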(event `self.ReceiveBeginPlay`
  (bind _returnvalue (`PrimitiveComponent.CreateDynamicMaterialInstance` (`self.StaticMesh`) 1 null "None"))
  (set `self.DynamicMaterialRef` _returnvalue)
  (`MediaPlayer.OpenSource` (`self.Video Source`) "/Game/DEV_Brian/Switches/Fish_Scene_Smaller_Resolution.Fish_Scene_Smaller_Resolution"))

(event `SetFishSceneActive`
  (`MaterialInstanceDynamic.SetScalarParameterValue` (`self.DynamicMaterialRef`) "FishSceneActive" 1.0)
  (`GameplayStatics.PlaySoundAtLocation` "/Game/Sounds/Fish/CUE_FishAlarm.CUE_FishAlarm" (`SceneComponent.K2_GetComponentLocation` (`self.StaticMesh`)) (struct) 1.0 1.0 0.0 null null null))

(event `SetFishSceneFalse`
  (`MaterialInstanceDynamic.SetScalarParameterValue` (`self.DynamicMaterialRef`) "FishSceneActive" 0.0))

(fn `UserConstructionScript`)