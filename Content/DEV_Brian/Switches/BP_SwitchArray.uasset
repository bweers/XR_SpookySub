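; BP_SwitchArray is an actor that groups nine child-actor BP_Switch instances into one switch panel.
; On BeginPlay it casts each child actor and adds it to SwitchesList, stopping at the first failed cast.
; TriggerFishEvent clears SwitchArrayState and sets each listed switch to a random state.
; CheckSwitchStates is an empty stub, so nothing in this graph evaluates the switch states.
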(event `self.ReceiveBeginPlay`
  (`self.CreateSwitchList`))

(fn `CheckSwitchStates`)

(fn `CreateSwitchList`
  (bind _asbp_switch (cast `/Game/DEV_Brian/Switches/BP_Switch` (`ChildActorComponent.ChildActor` (`self.Switch1`))))
  (`KismetArrayLibrary.Array_Add` (`self.SwitchesList`) _asbp_switch)
  (bind _asbp_switch_2 (cast `/Game/DEV_Brian/Switches/BP_Switch` (`ChildActorComponent.ChildActor` (`self.Switch2`))))
  (`KismetArrayLibrary.Array_Add` (`self.SwitchesList`) _asbp_switch_2)
  (bind _asbp_switch_3 (cast `/Game/DEV_Brian/Switches/BP_Switch` (`ChildActorComponent.ChildActor` (`self.Switch3`))))
  (`KismetArrayLibrary.Array_Add` (`self.SwitchesList`) _asbp_switch_3)
  (bind _asbp_switch_4 (cast `/Game/DEV_Brian/Switches/BP_Switch` (`ChildActorComponent.ChildActor` (`self.Switch4`))))
  (`KismetArrayLibrary.Array_Add` (`self.SwitchesList`) _asbp_switch_4)
  (bind _asbp_switch_5 (cast `/Game/DEV_Brian/Switches/BP_Switch` (`ChildActorComponent.ChildActor` (`self.Switch5`))))
  (`KismetArrayLibrary.Array_Add` (`self.SwitchesList`) _asbp_switch_5)
  (bind _asbp_switch_6 (cast `/Game/DEV_Brian/Switches/BP_Switch` (`ChildActorComponent.ChildActor` (`self.Switch6`))))
  (`KismetArrayLibrary.Array_Add` (`self.SwitchesList`) _asbp_switch_6)
  (bind _asbp_switch_7 (cast `/Game/DEV_Brian/Switches/BP_Switch` (`ChildActorComponent.ChildActor` (`self.Switch7`))))
  (`KismetArrayLibrary.Array_Add` (`self.SwitchesList`) _asbp_switch_7)
  (bind _asbp_switch_8 (cast `/Game/DEV_Brian/Switches/BP_Switch` (`ChildActorComponent.ChildActor` (`self.Switch8`))))
  (`KismetArrayLibrary.Array_Add` (`self.SwitchesList`) _asbp_switch_8)
  (bind _asbp_switch_9 (cast `/Game/DEV_Brian/Switches/BP_Switch` (`ChildActorComponent.ChildActor` (`self.Switch9`))))
  (`KismetArrayLibrary.Array_Add` (`self.SwitchesList`) _asbp_switch_9))

(fn `TriggerFishEvent`
  (set `self.SwitchArrayState` false)
  (for _array_element (`self.SwitchesList`)
    (`/Game/DEV_Brian/Switches/BP_Switch.SetState` _array_element (`KismetMathLibrary.RandomBool`))))

(fn `UserConstructionScript`)