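; BP_LaunchButton is a physical VR button that launches flares through its referenced switch array when a motion controller touches it.
; SetReadyForLaunch arms it, raising the button and lighting its state through a dynamic material parameter.
; An overlap by a component attached to a motion controller disarms it, calls FlaresLaunched, resets the material, sinks the button and plays a double click sound.
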(event `self.ReceiveBeginPlay`
  (bind _returnvalue (`PrimitiveComponent.CreateDynamicMaterialInstance` (`self.Button`) 0 "/Game/DEV_Brian/Imported/Button/MAT_Button_Inst.MAT_Button_Inst" "None"))
  (set `self.DynamicMaterial` _returnvalue))

(event `SetReadyForLaunch`
  (set `self.ReadyForLaunch` true)
  (`MaterialInstanceDynamic.SetScalarParameterValue` (`self.DynamicMaterial`) "State" 1.0)
  (`SceneComponent.K2_SetRelativeLocation` (`self.Button`) (0.0 0.0 0.0) false false))

(event `self.Collider.OnComponentBeginOverlap`
  (params (OverlappedComponent :type "PrimitiveComponent Object Reference") (OtherActor :type "Actor Object Reference") (OtherComp :type "PrimitiveComponent Object Reference") (OtherBodyIndex :type Integer) (bFromSweep :type Boolean) (SweepResult :type "HitResult Structure (by ref)"))
  (cast `MotionControllerComponent` (`SceneComponent.GetAttachParent` OtherComp)
    (:`then`
      (if (`self.ReadyForLaunch`)
        (set `self.ReadyForLaunch` false)
        (`/Game/DEV_Brian/Switches/BP_SwitchArray.FlaresLaunched` (`self.SwitchArrayRef`))
        (`MaterialInstanceDynamic.SetScalarParameterValue` (`self.DynamicMaterial`) "State" 0.0)
        (`SceneComponent.K2_SetRelativeLocation` (`self.Button`) (0.0 0.0 -13.0) false false)
        (`GameplayStatics.PlaySoundAtLocation` "/Game/Sounds/Buttons/CUE_ButtonClick.CUE_ButtonClick" (`SceneComponent.K2_GetComponentLocation` (`self.Button`)) (struct) 1.0 1.0 0.0 null null null)
        (`KismetSystemLibrary.Delay` 0.15)
        (`GameplayStatics.PlaySoundAtLocation` "/Game/Sounds/Buttons/CUE_ButtonClick.CUE_ButtonClick" (`SceneComponent.K2_GetComponentLocation` (`self.Button`)) (struct) 1.0 1.0 0.0 null null null)))
    (:`CastFailed`
      (`KismetSystemLibrary.PrintString` "CAST FAILED FOR BUTTON" true true (struct :`R` 1.0 :`G` 0.455961 :`A` 1.0)))))

(fn `UserConstructionScript`)