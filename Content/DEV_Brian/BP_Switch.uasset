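; BP_Switch is a toggle switch operated by touch from a motion controller, apparently for VR.
; When a component attached to a MotionControllerComponent begins overlapping the Box, a FlipFlop tilts the Cylinder to the opposite pitch and updates the SwitchState boolean.
; A DoOnce, reset after a quarter-second Delay, debounces overlaps.
; Other overlapping components that pass the DoOnce only print a cast-failure message.
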(event `self.ReceiveBeginPlay`
  (`SceneComponent.K2_SetRelativeRotation` (`self.Cylinder`) (struct :`Pitch` 20.0) false false))

(event `self.Box.OnComponentBeginOverlap`
  (params (OverlappedComponent :type "PrimitiveComponent Object Reference") (OtherActor :type "Actor Object Reference") (OtherComp :type "PrimitiveComponent Object Reference") (OtherBodyIndex :type Integer) (bFromSweep :type Boolean) (SweepResult :type "HitResult Structure (by ref)"))
  (`|ExecutionSequence`
    (:`then_0`
      (`/Engine/EditorBlueprintResources/StandardMacros.DoOnce` false :!label _label
        (:`Completed`
          (cast `MotionControllerComponent` (`SceneComponent.GetAttachParent` OtherComp)
            (:`then`
              (`/Engine/EditorBlueprintResources/StandardMacros.FlipFlop`
                (:`A`
                  (`SceneComponent.K2_SetRelativeRotation` (`self.Cylinder`) (struct :`Pitch` 20.0) false false)
                  (set `self.SwitchState` false))
                (:`B`
                  (`SceneComponent.K2_SetRelativeRotation` (`self.Cylinder`) (struct :`Pitch` -20.0) false false)
                  (set `self.SwitchState` true))))
            (:`CastFailed`
              (`KismetSystemLibrary.PrintString` "CAST FAILED" true true (struct :`R` 1.0 :`B` 0.038757 :`A` 1.0)))))))
    (:`then_1`
      (`KismetSystemLibrary.Delay` 0.25)
      (goto _label :!via `Reset`))))

(fn `UserConstructionScript`)