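; VHS monster prop that plays an eye video and swallows VHS tapes that touch its collider.
; A delayed Tick flickers its spotlight with randomly sampled Perlin noise.
; On overlap, it releases the tape from the player's grab, disables its physics and collision, and snaps it above the root.
; A timeline then animates the tape's height before destroying it and clearing HasTape for the next one.
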(event `self.ReceiveBeginPlay`
  (`MediaPlayer.OpenSource` (`self.VideoSource`) "/Game/VHS_Monster/VHS_EYE.VHS_EYE"))

(event `self.ReceiveTick`
  (params (DeltaSeconds :type "Float (single-precision)"))
  (`KismetSystemLibrary.Delay` (`KismetMathLibrary.RandomFloatInRange` 0.06 0.1))
  (`LightComponent.SetIntensity` (`self.SpotLight`) (`KismetAnimationLibrary.K2_MakePerlinNoiseAndRemap` (`KismetMathLibrary.RandomFloatInRange` -5.0 5.0) 100.0 300.0)))

(event `self.Collider.OnComponentBeginOverlap`
  (params (OverlappedComponent :type "PrimitiveComponent Object Reference") (OtherActor :type "Actor Object Reference") (OtherComp :type "PrimitiveComponent Object Reference") (OtherBodyIndex :type Integer) (bFromSweep :type Boolean) (SweepResult :type "HitResult Structure (by ref)"))
  (bind (_originalworldlocation_x _originalworldlocation_y _originalworldlocation_z) (`KismetMathLibrary.BreakVector` (`self.OriginalWorldLocation`)))
  (bind _returnvalue (+ (`SceneComponent.K2_GetComponentLocation` (`self.DefaultSceneRoot`)) (0.0 0.0 100.0)))
  (if (not (`self.HasTape`))
    (bind _asbp_vhs_tape (cast `/Game/DEV_Brian/BP_VhsTape` OtherActor)
      (:`then`
        (set `self.HasTape` true)
        (set `self.GrabbedVHSTape` _asbp_vhs_tape)
        (bind _breleased (`/Game/VRTemplate/Blueprints/GrabComponent.TryRelease` (`/Game/DEV_Brian/BP_VhsTape.GrabComponent` _asbp_vhs_tape)))
        (if _breleased
          (bind _staticmesh (`/Game/DEV_Brian/BP_VhsTape.StaticMesh` _asbp_vhs_tape))
          (`SceneComponent.K2_SetWorldLocationAndRotation` :`self` _staticmesh :`NewLocation` _returnvalue)
          (`PrimitiveComponent.SetSimulatePhysics` _staticmesh false)
          (`PrimitiveComponent.SetCollisionEnabled` _staticmesh "NoCollision")
          (set `self.OriginalWorldLocation` _returnvalue)
          ;[1 1 1] Animation for Tape
          (bind (_direction _z_value) (`Timeline|InsertAnim` :!via `PlayFromStart`)
            (:`Update`
              (`SceneComponent.K2_SetWorldLocation` (`/Game/DEV_Brian/BP_VhsTape.StaticMesh` (`self.GrabbedVHSTape`)) (`KismetMathLibrary.MakeVector` _originalworldlocation_x _originalworldlocation_y (+ _z_value _originalworldlocation_z)) false false))
            (:`Finished`
              (set `self.HasTape` false)
              (`self.K2_DestroyActor` (`self.GrabbedVHSTape`))))))
      (:`CastFailed`
        (`KismetSystemLibrary.PrintString` "CAST FAILED")))))

(fn `Try Grab`
  (params (MotionController :type "MotionControllerComponent Object Reference"))
  (returns (SpawnedActorGrabComponent :type "/Game/VRTemplate/Blueprints/GrabComponent Object Reference")))

(fn `UserConstructionScript`)