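; BP_BreakerLever is a VR breaker switch lever that a motion controller grabs to flip between two snapped states.
; Attaching unpauses a looping timer that pitches BreakerSwitch toward the controller via look-at rotation, clamped to ±SnapAngle.
; Once detached, the still-running timer snaps the switch to the nearer limit by pitch sign and updates LeverState.
; SetState places the lever directly and starts it in the true (negative pitch) position on BeginPlay.
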(event `PauseTimer`)

(event `ResumeTimer`)

(event `self.ReceiveBeginPlay`
  (bind _returnvalue (`KismetSystemLibrary.K2_SetTimerDelegate` (delegate `UpdatePosition`) 0.01 true))
  (bind _output_get (set `self.UpdatePositionTimer` _returnvalue))
  (`KismetSystemLibrary.K2_PauseTimerHandle` _output_get)
  (`self.SetState` true))

(event `UpdatePosition`
  (bind _snapangle (`self.SnapAngle`))
  (bind _breakerswitch (`self.BreakerSwitch`))
  (bind (_returnvalue_roll _returnvalue_pitch _returnvalue_yaw) (`KismetMathLibrary.BreakRotator` (`SceneComponent.K2_GetComponentRotation` _breakerswitch)))
  (bind (_returnvalue_roll_2 _returnvalue_pitch_2) (`KismetMathLibrary.BreakRotator` (`KismetMathLibrary.FindLookAtRotation` (`SceneComponent.K2_GetComponentLocation` (`self.Root`)) (`SceneComponent.K2_GetComponentLocation` (`self.AttachedMotionController`)))))
  (if (`self.Attached`)
    ;[1 1 1] Implement snapping code here
    (if true
      (`SceneComponent.K2_SetWorldRotation` _breakerswitch (`KismetMathLibrary.MakeRotator` _returnvalue_roll (`KismetMathLibrary.ClampAngle` _returnvalue_pitch_2 (* _snapangle -1.0) _snapangle) _returnvalue_yaw) false false))
    (elif (>= (.pitch (`SceneComponent.RelativeRotation` (`self.BreakerSwitch`))) 0.0)
      (`SceneComponent.K2_SetRelativeRotation` (`self.BreakerSwitch`) (`KismetMathLibrary.MakeRotator` 0.0 (`self.SnapAngle`)) false false)
      (set `self.LeverState` false)
      (else
        (`SceneComponent.K2_SetRelativeRotation` (`self.BreakerSwitch`) (`KismetMathLibrary.MakeRotator` 0.0 (* (`self.SnapAngle`) -1.0)) false false)
        (set `self.LeverState` true)))))

(fn `Attach to Controller`
  (params (MotionController :type "MotionControllerComponent Object Reference"))
  (set `self.Attached` true)
  (set `self.AttachedMotionController` MotionController)
  (`KismetSystemLibrary.K2_UnPauseTimerHandle` (`self.UpdatePositionTimer`)))

(fn `Detach from Controller`
  (params (MotionController :type "MotionControllerComponent Object Reference"))
  (set `self.Attached` false)
  (set `self.AttachedMotionController` null))

(fn `SetState`
  (params (NewState :type Boolean))
  (if NewState
    (`SceneComponent.K2_SetRelativeRotation` (`self.BreakerSwitch`) (`KismetMathLibrary.MakeRotator` 0.0 (* (`self.SnapAngle`) -1.0)) false false)
    (set `self.LeverState` true)
    (else
      (`SceneComponent.K2_SetRelativeRotation` (`self.BreakerSwitch`) (`KismetMathLibrary.MakeRotator` 0.0 (`self.SnapAngle`)) false false)
      (set `self.LeverState` false))))

(fn `UserConstructionScript`)