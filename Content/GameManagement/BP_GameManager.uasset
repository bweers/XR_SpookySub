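; BP_GameManager runs the game loop: survive a countdown shown on a clock while tending a breaker box, switch array and VHS monster.
; Staggered one-second looping timers drive the countdown and each hazard's counters.
; Each hazard triggers trouble after its cycle time and calls GameLose if left bad too long.
; Countdown expiry only prints a win; GameLose is empty, with its fade and LoseLevel load disconnected.
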(event `self.ReceiveBeginPlay`
  (bind _returnvalue (`KismetSystemLibrary.K2_SetTimerDelegate` (`|CreateDelegate` :!event `GameTimer`) 1.0 true))
  (set `self.GameTimerRef` _returnvalue)
  (bind _returnvalue_2 (`KismetSystemLibrary.K2_SetTimerDelegate` (`|CreateDelegate` :!event `BreakerBoxTimer`) 1.0 true 1.0))
  (set `self.BreakerBoxTimerRef` _returnvalue_2)
  (bind _returnvalue_3 (`KismetSystemLibrary.K2_SetTimerDelegate` (`|CreateDelegate` :!event `SwitchArrayTimer`) 1.0 true 2.0))
  (set `self.SwitchArrayTimerRef` _returnvalue_3)
  (bind _returnvalue_4 (`KismetSystemLibrary.K2_SetTimerDelegate` (`|CreateDelegate` :!event `VHSTimer`) 1.0 true 3.0))
  (set `self.VHSTimerRef` _returnvalue_4)
  (set `self.CurrentTimeLeft` (`self.TimeLimit`)))

(event `GameTimer`
  (bind (_days _hours _minutes _seconds) (`KismetMathLibrary.BreakTimespan` (`self.CurrentTimeLeft`)))
  (bind (_days_2 _hours_2 _minutes_2 _seconds_2) (`KismetMathLibrary.BreakTimespan` (`self.GameTimespan`)))
  ;[0.2083 0.2083 0.2083] Deprecated
  (bind _result (`/Engine/EditorBlueprintResources/StandardMacros.IncrementInt` _seconds_2)
    (:`  `
      (set `self.GameTimespan` (`KismetMathLibrary.MakeTimespan` 0 0 _minutes_2 _result))
      (if (not (`self.GameWon`))
        (bind _result_2 (`/Engine/EditorBlueprintResources/StandardMacros.DecrementInt` _seconds)
          (:`  `
            (bind _output_get (set `self.CurrentTimeLeft` (`KismetMathLibrary.MakeTimespan` 0 0 _minutes _result_2)))
            (`/Game/Clock/BP_Clock.SetTime` (`self.ClockRef`) _output_get)
            ;[0.4642 1 0.4223] Win Condition
            (if (<= _output_get (`KismetMathLibrary.MakeTimespan` 0))
              (`self.GameWin`))))))))

(event `BreakerBoxTimer`
  (if (`/Game/DEV_Brian/BP_BreakerBox.BreakerBoxState` (`self.BreakerBox_Ref`))
    (set `self.BreakerBox_BadState_Counter` 0)
    (bind _result (`/Engine/EditorBlueprintResources/StandardMacros.IncrementInt` (`self.BreakerBox_Cycle_Counter`))
      (:`  `
        (if (>= _result (`self.BreakerBox_Cycle_Time`))
          (`/Game/DEV_Brian/BP_BreakerBox.SetBroken` (`self.BreakerBox_Ref`)))))
    (else
      (set `self.BreakerBox_Cycle_Counter` 0)
      (bind _result_2 (`/Engine/EditorBlueprintResources/StandardMacros.IncrementInt` (`self.BreakerBox_BadState_Counter`))
        (:`  `
          (if (>= _result_2 (`self.BreakerBox_BadState_MaxTime`))
            ;[1 0.5852 0.7822] Lose Condition
            (`/Engine/EditorBlueprintResources/StandardMacros.DoOnce` false :!label _label
              (:`Completed`
                (`self.GameLose`)
                (`KismetSystemLibrary.PrintString` "GAME LOSE TRIGGERED" true true (struct :`R` 1.0 :`G` 0.014665 :`A` 1.0) 20.0)))))))))

(event `SwitchArrayTimer`
  (if (`/Game/DEV_Brian/Switches/BP_SwitchArray.SwitchArrayState` (`self.SwitchArray_Ref`))
    (set `self.SwitchArray_BadState_Counter` 0)
    (bind _result (`/Engine/EditorBlueprintResources/StandardMacros.IncrementInt` (`self.SwitchArray_Cycle_Counter`))
      (:`  `
        (if (>= _result (`self.SwitchArray_Cycle_Time`))
          (`/Game/DEV_Brian/Switches/BP_SwitchArray.TriggerFishEvent` (`self.SwitchArray_Ref`)))))
    (else
      (set `self.SwitchArray_Cycle_Counter` 0)
      (bind _result_2 (`/Engine/EditorBlueprintResources/StandardMacros.IncrementInt` (`self.SwitchArray_BadState_Counter`))
        (:`  `
          (if (>= _result_2 (`self.SwitchArray_BadState_MaxTime`))
            (goto _label)))))))

(event `VHSTimer`
  (if (`/Game/DEV_Brian/BP_VhsMonster.VHSMonster_State` (`self.VHSMonster_Ref`))
    (set `self.VHS_Badstate_Counter` 0)
    (bind _result (`/Engine/EditorBlueprintResources/StandardMacros.IncrementInt` (`self.VHS_Cycle_Counter`))
      (:`  `
        (if (>= _result (`self.VHS_Cycle_Time`))
          (`/Game/DEV_Brian/BP_VhsMonster.SetHunger` (`self.VHSMonster_Ref`) true))))
    (else
      (set `self.VHS_Cycle_Counter` 0)
      (bind _result_2 (`/Engine/EditorBlueprintResources/StandardMacros.IncrementInt` (`self.VHS_Badstate_Counter`))
        (:`  `
          (if (>= _result_2 (`self.VHS_BadState_MaxTime`))
            (goto _label)))))))

(event `GameLose`)

(event `GameWin`
  (if (not (`self.GameLost`))
    (set `self.GameWon` true)
    (`KismetSystemLibrary.PrintString` "GAME WIN" true true (struct :`G` 1.0 :`B` 0.084032 :`A` 1.0) 10.0)))

(fn `UserConstructionScript`)