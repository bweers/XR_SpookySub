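; VHS monster with an eye video and flickering spotlight that is fed grabbable VHS tapes.
; An overlapping tape is released from the controller's grip, snapped to the slot, slid in by a timeline and destroyed, clearing hunger.
; SetHunger blends the dynamic screen material and swaps between normal and harsh static loops, though only the fed state is triggered here.
; Tick uses a random Delay and Perlin noise to flicker the light.
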(event `self.ReceiveBeginPlay`
  (`MediaPlayer.OpenSource` (`self.VideoSource`) "/Game/VHS_Monster/VHS_EYE.VHS_EYE")
  (bind _returnvalue (`PrimitiveComponent.CreateDynamicMaterialInstance` (`self.StaticMesh`) 1 "/Game/VHS_Monster/MAT_VHS_Screen_Inst.MAT_VHS_Screen_Inst" "None"))
  (set `self.Dynamic VHS Material` _returnvalue)
  (bind _returnvalue_2 (`GameplayStatics.SpawnSoundAttached` "/Game/Sounds/VHS/CUE_tv_Static.CUE_tv_Static" (`self.StaticMesh`) "None" (0.0 0.0 0.0) (struct) "KeepRelativeOffset" false 1.0 1.0 0.0 null null false))
  (set `self.NormalStatic` _returnvalue_2)
  (bind _returnvalue_3 (`GameplayStatics.SpawnSoundAttached` "/Game/Sounds/VHS/CUE_tvStatic_harsh.CUE_tvStatic_harsh" (`self.Collider`) "None" (0.0 0.0 0.0) (struct) "KeepRelativeOffset" false 0.2 1.0 0.0 null null false))
  (set `self.HarshStatic` _returnvalue_3))

(event `self.ReceiveTick`
  (params (DeltaSeconds :type "Float (single-precision)"))
  (`KismetSystemLibrary.Delay` (`KismetMathLibrary.RandomFloatInRange` 0.06 0.1))
  (`LightComponent.SetIntensity` (`self.SpotLight`) (`KismetAnimationLibrary.K2_MakePerlinNoiseAndRemap` (`KismetMathLibrary.RandomFloatInRange` -5.0 5.0) 100.0 300.0)))

(event `self.Collider.OnComponentBeginOverlap`
  (params (OverlappedComponent :type "PrimitiveComponent Object Reference") (OtherActor :type "Actor Object Reference") (OtherComp :type "PrimitiveComponent Object Reference") (OtherBodyIndex :type Integer) (bFromSweep :type Boolean) (SweepResult :type "HitResult Structure (by ref)"))
  (if (not (`self.HasTape`))
    (bind _asbp_vhs_tape (cast `/Game/VHS_Monster/BP_VhsTape` OtherActor)
      (:`then`
        (`self.RemoveTapeFromController` _asbp_vhs_tape)
        (`GameplayStatics.PlaySoundAtLocation` "/Game/Sounds/VHS/CUE_VHS_Insert.CUE_VHS_Insert" (`SceneComponent.K2_GetComponentLocation` (`self.Collider`)) (struct) 1.0 1.0 0.0 null null null)
        ;[1 1 1] Animation for Tape
        (bind (_direction _z_value) (`Timeline|InsertAnim` :!via `PlayFromStart`)
          (:`Update`
            (`SceneComponent.K2_SetWorldLocation` (`/Game/VHS_Monster/BP_VhsTape.StaticMesh` (`self.GrabbedVHSTape`)) (`KismetMathLibrary.VLerp` (`SceneComponent.K2_GetComponentLocation` (`self.TapeSetPoint`)) (`SceneComponent.K2_GetComponentLocation` (`self.TapeEndPoint`)) _z_value) false false))
          (:`Finished`
            (set `self.HasTape` false)
            (`self.K2_DestroyActor` (`self.GrabbedVHSTape`))
            (`self.SetHunger` false))))
      (:`CastFailed`
        (`KismetSystemLibrary.PrintString` "CAST FAILED")))))

(fn `RemoveTapeFromController`
  (params (GrabbedVHSTape :type "/Game/VHS_Monster/BP_VhsTape Object Reference"))
  (bind _staticmesh (`/Game/VHS_Monster/BP_VhsTape.StaticMesh` GrabbedVHSTape))
  (bind _location (.location (`SceneComponent.K2_GetComponentToWorld` (`self.TapeSetPoint`))))
  (set `self.HasTape` true)
  (set `self.GrabbedVHSTape` GrabbedVHSTape)
  (bind _breleased (`/Game/VRTemplate/Blueprints/GrabComponent.TryRelease` (`/Game/VHS_Monster/BP_VhsTape.GrabComponent` GrabbedVHSTape)))
  (if _breleased
    (`SceneComponent.K2_SetWorldTransform` _staticmesh (`KismetMathLibrary.MakeTransform` _location (`KismetMathLibrary.MakeRotator` (.roll (.rotation (`SceneComponent.K2_GetComponentToWorld` (`self.TapeSetPoint`)))) (.pitch (.rotation (`SceneComponent.K2_GetComponentToWorld` (`self.TapeSetPoint`)))) (+ (.yaw (.rotation (`SceneComponent.K2_GetComponentToWorld` (`self.TapeSetPoint`)))) 90.0))) false false)
    (`PrimitiveComponent.SetSimulatePhysics` _staticmesh false)
    (`PrimitiveComponent.SetCollisionEnabled` _staticmesh "NoCollision")
    (set `self.OriginalWorldLocation` _location)))

(fn `SetHunger`
  (params (`New Hunger State` :type Boolean))
  (if `New Hunger State`
    (set `self.VHSMonster_State` false)
    (`MaterialInstanceDynamic.SetScalarParameterValue` (`self.Dynamic VHS Material`) "HungerAmountLerp" 0.8)
    (`AudioComponent.SetVolumeMultiplier` (`self.NormalStatic`) 0.0)
    (`AudioComponent.SetVolumeMultiplier` (`self.HarshStatic`) 1.0)
    (else
      (set `self.VHSMonster_State` true)
      (`MaterialInstanceDynamic.SetScalarParameterValue` (`self.Dynamic VHS Material`) "HungerAmountLerp" 0.0)
      (`AudioComponent.SetVolumeMultiplier` (`self.NormalStatic`) 1.0)
      (`AudioComponent.SetVolumeMultiplier` (`self.HarshStatic`) 0.0))))

(fn `Try Grab`
  (params (MotionController :type "MotionControllerComponent Object Reference"))
  (returns (SpawnedActorGrabComponent :type "/Game/VRTemplate/Blueprints/GrabComponent Object Reference")))

(fn `UserConstructionScript`)