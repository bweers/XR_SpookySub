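; BP_Clock is an in-game clock that displays a game timer's minutes and seconds through a TextRender component.
; Its SetTime event takes a GameTimer value, builds a colon-separated string and writes it to the text; the Blueprint does no timekeeping itself.
; Seconds below ten get a leading zero, while minutes are always prefixed with a zero regardless of value.
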(event `SetTime`
  (params (GameTimer :type "Timespan Structure"))
  (bind (_days _hours _minutes _seconds) (`KismetMathLibrary.BreakTimespan` GameTimer))
  (bind (_days_2 _hours_2 _minutes_2 _seconds_2) (`KismetMathLibrary.BreakTimespan` GameTimer))
  (if (< _seconds_2 10)
    (`TextRenderComponent.K2_SetText` (`self.TextRender`) (`KismetTextLibrary.Conv_StringToText` (`KismetStringLibrary.Concat_StrStr` "0" (`KismetStringLibrary.Conv_IntToString` _minutes) ":" "0" (`KismetStringLibrary.Conv_IntToString` _seconds))))
    (else
      (`TextRenderComponent.K2_SetText` (`self.TextRender`) (`KismetTextLibrary.Conv_StringToText` (`KismetStringLibrary.Concat_StrStr` "0" (`KismetStringLibrary.Conv_IntToString` _minutes_2) ":" (`KismetStringLibrary.Conv_IntToString` _seconds_2)))))))

(fn `UserConstructionScript`)